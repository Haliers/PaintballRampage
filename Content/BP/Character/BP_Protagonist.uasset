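; Player character Blueprint that handles death presentation, landing damage and pickup of five colors of ammo.
; On death, it swaps the main camera for a repositioned death camera and triggers the death screen on BP_HUD.
; Landing applies jump ability damage to every enemy inside DamageSphere.
; Capsule overlaps with ammo drops add to the matching color reserve and destroy the drop, while a helper function copies reserves to the screen widget.
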(event OnComponentBeginOverlap(CapsuleComponent)
  (params (OverlappedComponent :type Primitive%20Component%20Object%20Reference) (OtherActor :type Actor%20Object%20Reference) (OtherComp :type Primitive%20Component%20Object%20Reference) (OtherBodyIndex :type Integer) (bFromSweep :type Boolean) (SweepResult :type Hit%20Result%20Structure%20%28by%20ref%29))
  (bind _asbp_ammo_drop (Utilities|Casting|CastToBP_AmmoDrop OtherActor))
  (Utilities|FlowControl|Sequence
    (:then_0
      (switch Utilities|FlowControl|Switch|SwitchonEDropColor (Variables|/Script/PaintballRampage.AmmoDrop|GetDropColor _asbp_ammo_drop)
        (:EDC_Purple
          (Class|Protagonist|AddPurpleAmmoReserve (Variables|/Script/PaintballRampage.AmmoDrop|GetAmmo _asbp_ammo_drop)))
        (:EDC_Yellow
          (Class|Protagonist|AddYellowAmmoReserve (Variables|/Script/PaintballRampage.AmmoDrop|GetAmmo _asbp_ammo_drop)))
        (:EDC_Green
          (Class|Protagonist|AddGreenAmmoReserve (Variables|/Script/PaintballRampage.AmmoDrop|GetAmmo _asbp_ammo_drop)))
        (:EDC_Blue
          (Class|Protagonist|AddBlueAmmoReserve (Variables|/Script/PaintballRampage.AmmoDrop|GetAmmo _asbp_ammo_drop)))
        (:EDC_Red
          (Class|Protagonist|AddRedAmmoReserve (Variables|/Script/PaintballRampage.AmmoDrop|GetAmmo _asbp_ammo_drop)))))
    (:then_1
      (Actor|DestroyActor _asbp_ammo_drop))))

(event EventDeathSetupBlueprint
  (bind _deathcamera (Variables|Default|GetDeathCamera))
  (Utilities|Casting|CastToBP_HUD (HUD|GetHUD (Game|GetPlayerController 0)))
  (Components|Activation|SetActive (Variables|Default|GetCameraComponent) false false)
  (Components|Activation|SetActive _deathcamera true false)
  (Transformation|SetWorldTransform _deathcamera (Variables|Default|GetDeathCameraTransform) false false)
  (bind _asbp_hud (Utilities|Casting|CastToBP_HUD (HUD|GetHUD (Game|GetPlayerController 0))))
  (Default|DeathHUD _asbp_hud))

(event EventOnLanded
  (params (Hit :type Hit%20Result%20Structure%20%28by%20ref%29))
  (for _array_element (Collision|GetOverlappingActors (Variables|Default|GetDamageSphere) "/Game/BP/Enemy/BP_BaseEnemy.BP_BaseEnemy_C" :!class /Script/Engine.PrimitiveComponent)
    (bind _asbp_base_enemy (Utilities|Casting|CastToBP_BaseEnemy _array_element)
      (:then
        (Class|BaseEnemy|ApplyDamage _asbp_base_enemy (Variables|Default|GetJumpAbilityDamage)))
      (:CastFailed
        (Development|PrintString "failed")))))

(event EventBeginPlay
  (Components|Activation|SetActive (Variables|Default|GetDeathCamera) false false))

(fn ConstructionScript)

(fn SetReserveAmmoWidget
  (bind _screenwidget (Variables|Default|GetScreenWidget))
  (bind _returnvalue (Class|Protagonist|GetPurpleAmmoReserve))
  (Variables|/Game/BP/Widget/WBP_Screen.WBP_Screen_C|SetPurpleAmmo _screenwidget _returnvalue)
  (bind _returnvalue_2 (Class|Protagonist|GetYellowAmmoReserve))
  (Variables|/Game/BP/Widget/WBP_Screen.WBP_Screen_C|SetYellowAmmo _screenwidget _returnvalue_2)
  (bind _returnvalue_3 (Class|Protagonist|GetBlueAmmoReserve))
  (Variables|/Game/BP/Widget/WBP_Screen.WBP_Screen_C|SetBlueAmmo _screenwidget _returnvalue_3)
  (bind _returnvalue_4 (Class|Protagonist|GetGreenAmmoReserve))
  (Variables|/Game/BP/Widget/WBP_Screen.WBP_Screen_C|SetGreenAmmo _screenwidget _returnvalue_4)
  (bind _returnvalue_5 (Class|Protagonist|GetRedAmmoReserve))
  (Variables|/Game/BP/Widget/WBP_Screen.WBP_Screen_C|SetRedAmmo _screenwidget _returnvalue_5))

(fn GetHitResultOfCamera)