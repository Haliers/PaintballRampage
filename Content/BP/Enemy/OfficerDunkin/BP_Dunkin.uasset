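; BP_Dunkin is the Officer Dunkin enemy Blueprint, adding a donut-throwing ranged attack.
; Its ThrowDonut event spawns a BP_Donut at the mesh's ThrowSocket, facing the actor's rotation and ignoring spawn collisions.
; It then passes damage, decal size, a primary-color material and the enemy's linear color to the donut, so each projectile matches its thrower.
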(event Custom|Throw%20Donut
  (bind _returnvalue (Game|SpawnActorfromClass "/Game/BP/Enemy/OfficerDunkin/BP_Donut.BP_Donut_C" (Math|Transform|MakeTransform (Transformation|GetSocketLocation (Variables|Character|GetMesh) "ThrowSocket") (Transformation|GetActorRotation)) "AlwaysSpawn" 0 0))
  (Class|AProjectile|SetDamage _returnvalue (Variables|Default|GetDamage))
  (Class|AProjectile|SetDecalSize _returnvalue "5.000000,50.000000,50.000000")
  (bind _returnvalue_2 (Class|BaseEnemy|GetPrimaryColor))
  (Rendering|Material|SetMaterial (Variables|/Game/BP/Enemy/OfficerDunkin/BP_Donut.BP_Donut_C|GetDonut _returnvalue) 0 _returnvalue_2)
  (Class|AProjectile|SetLinearColor _returnvalue (Variables|Default|GetEnemyLinearColor)))

(event EventBeginPlay
  (|CallParentFunction) ; This node is disabled and will not be called.\nDrag off pins to build functionality.
)

(event Collision|EventActorBeginOverlap
  (params (OtherActor :type Actor%20Object%20Reference))
  (|CallParentFunction OtherActor) ; This node is disabled and will not be called.\nDrag off pins to build functionality.
)

(event EventTick
  (params (DeltaSeconds :type Float%20%28single-precision%29))
  (|CallParentFunction DeltaSeconds) ; This node is disabled and will not be called.\nDrag off pins to build functionality.
)

(fn ConstructionScript
  (|CallParentFunction))