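; Explosive donut for the Officer Dunkin enemy that bursts when its Donut component hits something.
; On hit it attaches a paint decal to the hit component and spawns a colour-parameterised explosion, both placed at world Z zero with an upward normal computed for the decal.
; It then damages the first BP_Protagonist overlapping its Sphere, making the hit an area check, and destroys itself.
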(event OnComponentHit(Donut)
  (params (HitComponent :type Primitive%20Component%20Object%20Reference) (OtherActor :type Actor%20Object%20Reference) (OtherComp :type Primitive%20Component%20Object%20Reference) (NormalImpulse :type Vector :default "0, 0, 0") (Hit :type Hit%20Result%20Structure%20%28by%20ref%29))
  (bind (_bblockinghit _binitialoverlap _time _distance _location _impactpoint _normal _impactnormal _physmat _hitactor _hitcomponent) (Collision|BreakHitResult Hit))
  (bind _sphere (Variables|Default|GetSphere))
  (bind _overlappingactors (Collision|GetOverlappingActors _sphere "/Game/BP/Character/BP_Protagonist.BP_Protagonist_C" :!class /Script/Engine.PrimitiveComponent))
  (bind (_x _y) (Math|Vector|BreakVector _impactpoint))
  (bind _returnvalue (Math|Vector|MakeVector _x _y 0.0))
  (bind _returnvalue_2 (Math|Vector|MakeVector _x _y 1.0))
  (bind _output (Utilities|Array|Get(acopy) _overlappingactors))
  (bind _returnvalue_3 (- _returnvalue_2 _returnvalue))
  (Class|AProjectile|SpawnDecalatHitLocation _returnvalue _returnvalue_3 _hitcomponent)
  (Class|AProjectile|SpawnImpactFX _returnvalue _returnvalue_3)
  (Utilities|FlowControl|Sequence
    (:then_0
      (Utilities|IsValid _output
        (:Is%20Valid
          (bind _asbp_protagonist (Utilities|Casting|CastToBP_Protagonist _output))
          (Class|Protagonist|ApplyDamage _asbp_protagonist (Variables|Default|GetDamage)))))
    (:then_1
      (Actor|DestroyActor))))

(event EventBeginPlay)

(event Collision|EventActorBeginOverlap
  (params (OtherActor :type Actor%20Object%20Reference)))

(event EventTick
  (params (DeltaSeconds :type Float%20%28single-precision%29)))

(event EventSpawnDecalatHitLocation
  (params (ImpactLocation :type Vector :default "0, 0, 0") (ImpactNormal :type Vector :default "0, 0, 0") (AttachComponent :type Primitive%20Component%20Object%20Reference))
  (bind _returnvalue (Math|Rotator|MakeRotfromY ImpactNormal))
  (bind (_roll _pitch _yaw) (Math|Rotator|BreakRotator _returnvalue))
  (Class|GameplayStatics|SpawnDecalAttached (Variables|Default|GetDynamicPaintMaterial) (Variables|Default|GetDecalSize) 0 "None" ImpactLocation (Math|Rotator|MakeRotator _roll (- _pitch 9e+01) _yaw) "KeepRelativeOffset" 0.0))

(event EventSpawnImpactFX
  (params (ImpactLocation :type Vector :default "0, 0, 0") (ImpactNormal :type Vector :default "0, 0, 0"))
  (bind _returnvalue (Niagara|SpawnSystematLocation "/Game/Assets/VFX/Explosion/E_Explosion_System.E_Explosion_System" ImpactLocation (Math|Rotator|MakeRotator 0.0 0.0 0.0)))
  (Effects|Components|ParticleSystem|SetColorParameter _returnvalue "Color" (Variables|Default|GetLinearColor)))

(fn ConstructionScript)