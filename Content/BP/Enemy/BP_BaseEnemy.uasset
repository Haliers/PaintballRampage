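; Base enemy Blueprint providing a melee attack and a death sequence.
; Melee line-traces a short distance forward and applies Damage when it hits BP_Protagonist.
; ExecuteDeathProcess spawns a Niagara splash tinted with the enemy color, leaves death decals, calls Drop and destroys the actor.
; Decals come from a downward trace, with random sizes and a random number of extra scattered splats around the impact point.
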(event Custom|Melee
  (bind _returnvalue (Transformation|GetActorLocation))
  (bind _outhit (Collision|LineTraceByChannel _returnvalue (+ _returnvalue (* (Transformation|GetActorForwardVector) "125.000000,125.000000,125.000000")) "TraceTypeQuery4" false 0 "None" true "(R=1.000000,G=0.000000,B=0.000000,A=1.000000)" "(R=0.000000,G=1.000000,B=0.000000,A=1.000000)" 1.0))
  (bind _asbp_protagonist (Utilities|Casting|CastToBP_Protagonist (.HitActor (Collision|BreakHitResult _outhit))))
  (Class|Protagonist|ApplyDamage _asbp_protagonist (Variables|Default|GetDamage)))

(event EventBeginPlay)

(event Collision|EventActorBeginOverlap
  (params (OtherActor :type Actor%20Object%20Reference)))

(event EventTick
  (params (DeltaSeconds :type Float%20%28single-precision%29)))

(event EventExecuteDeathProcess
  (CallFunction|SpawnSplash)
  (CallFunction|SpawnDeathDecal)
  (Class|BaseEnemy|Drop)
  (Actor|DestroyActor))

(fn ConstructionScript)

(fn SpawnDeathDecal
  (bind _returnvalue (Transformation|GetActorLocation))
  (bind (_x _y _z) (Math|Vector|BreakVector _returnvalue))
  (bind _outhit (Collision|LineTraceByChannel _returnvalue (Math|Vector|MakeVector _x _y (- _z 5e+02)) "TraceTypeQuery1" false 0 "None"))
  (CallFunction|SpawnDecalwithRandomSize _outhit (.ImpactPoint (Collision|BreakHitResult _outhit)))
  (for _index (range 0 (Math|Random|RandomInteger 4))
    (bind _returnvalue_2 (CallFunction|GetRandomPoint (.ImpactPoint (Collision|BreakHitResult _outhit)) 75.0))
    (CallFunction|SpawnDecalwithRandomSize _outhit _returnvalue_2)))

(fn SpawnSplash
  (bind _returnvalue (Transformation|GetActorTransform))
  (bind (_location _rotation) (Math|Transform|BreakTransform _returnvalue))
  (bind _returnvalue_2 (Niagara|SpawnSystematLocation "/Game/Assets/VFX/Splash/N_DeathSplash_System.N_DeathSplash_System" _location _rotation))
  (Effects|Components|ParticleSystem|SetColorParameter _returnvalue_2 "Color" (Variables|Default|GetEnemyLinearColor)))

(fn SpawnDecalwithRandomSize
  (params (Hit :type Hit%20Result%20Structure%20%28by%20ref%29) (Location :type Vector))
  (bind (_bblockinghit _binitialoverlap _time _distance _location _impactpoint _normal _impactnormal _physmat _hitactor _hitcomponent) (Collision|BreakHitResult Hit))
  (bind _returnvalue (Math|Random|RandomFloatinRange 2e+01 1.5e+02))
  (bind _returnvalue_2 (Math|Rotator|MakeRotfromY _normal))
  (bind (_roll _pitch _yaw) (Math|Rotator|BreakRotator _returnvalue_2))
  (Class|GameplayStatics|SpawnDecalAttached (Variables|Default|GetDeathDecal) (Math|Vector|MakeVector 5.0 _returnvalue _returnvalue) _hitcomponent "None" Location (Math|Rotator|MakeRotator _roll (- _pitch 9e+01) _yaw) "KeepRelativeOffset" 0.0))

(fn GetRandomPoint
  (params (Origin :type Vector) (Radius :type Float%20%28double-precision%29))
  (bind _returnvalue (* Radius -1.0))
  (return (+ Origin (Math|Vector|MakeVector (Math|Random|RandomFloatinRange _returnvalue Radius) (Math|Random|RandomFloatinRange _returnvalue Radius) 0.0))))