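; Glock weapon Blueprint that supplies shot visuals: bullet tracers, impact effects and dynamic paint decals.
; The tracer spawns a Niagara system at the muzzle, with power and particle count scaled from Damage.
; Tracer and impact systems share one color parameter, and the impact aligns to the surface normal.
; Decals attach to the hit component, through either an event or a duplicate function taking a Hit.
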(event EventSpawnDecalatHitLocation
  (params (ImpactLocation :type Vector :default "0, 0, 0") (ImpactNormal :type Vector :default "0, 0, 0") (AttachComponent :type Primitive%20Component%20Object%20Reference))
  (bind _returnvalue (Math|Rotator|MakeRotfromY ImpactNormal))
  (bind (_roll _pitch _yaw) (Math|Rotator|BreakRotator _returnvalue))
  (Class|GameplayStatics|SpawnDecalAttached (Variables|Default|GetDynamicPaintMaterial) (Variables|Default|GetDecalSize) AttachComponent "None" ImpactLocation (Math|Rotator|MakeRotator _roll (- _pitch 9e+01) _yaw) "KeepRelativeOffset" 0.0))

(event EventSpawnImpactFX
  (params (ImpactLocation :type Vector :default "0, 0, 0") (ImpactNormal :type Vector :default "0, 0, 0"))
  (bind _returnvalue (Niagara|SpawnSystematLocation "/Game/Assets/VFX/Impact/N_Impact_System1.N_Impact_System1" ImpactLocation (Math|Conversions|RotationFromXVector ImpactNormal)))
  (Effects|Components|ParticleSystem|SetColorParameter _returnvalue "Color" (Variables|Default|GetLinearColor)))

(event EventSpawnTracer
  (bind _muzzlescenecomponent (Variables|Default|GetMuzzleSceneComponent))
  (bind _damage (Variables|Default|GetDamage))
  (bind _returnvalue (Niagara|SpawnSystematLocation "/Game/Assets/VFX/Tracer/N_Bullet_System.N_Bullet_System" (Transformation|GetWorldLocation _muzzlescenecomponent) (Transformation|GetWorldRotation _muzzlescenecomponent)))
  (Effects|Components|ParticleSystem|SetColorParameter _returnvalue "Color" (Variables|Default|GetLinearColor))
  (Effects|Components|ParticleSystem|SetFloatParameter _returnvalue "Power" (* _damage 5.0))
  (Effects|Components|ParticleSystem|SetIntParameter _returnvalue "ParticleNumber" (Math|Float|Truncate (/ _damage 2.0))))

(fn ConstructionScript)

(fn SpawnDecal
  (params (Hit :type Hit%20Result%20Structure))
  (bind (_bblockinghit _binitialoverlap _time _distance _location _impactpoint _normal _impactnormal _physmat _hitactor _hitcomponent) (Collision|BreakHitResult Hit))
  (bind _returnvalue (Math|Rotator|MakeRotfromY _normal))
  (bind (_roll _pitch _yaw) (Math|Rotator|BreakRotator _returnvalue))
  (Class|GameplayStatics|SpawnDecalAttached (Variables|Default|GetDynamicPaintMaterial) (Variables|Default|GetDecalSize) _hitcomponent "None" _location (Math|Rotator|MakeRotator _roll (- _pitch 9e+01) _yaw) "KeepRelativeOffset" 0.0))