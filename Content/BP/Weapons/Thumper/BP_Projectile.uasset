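; Thumper weapon grenade projectile that explodes on hit, damaging nearby enemies and leaving a paint decal.
; On impact it spawns a Niagara explosion, applies damage to every BP_BaseEnemy overlapping its Sphere, then destroys itself.
; The decal attaches to the hit component but is flattened to world Z=0 with a constant up normal, ignoring the actual surface height and orientation.
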(event OnComponentHit(ThumperGrenade)
  (params (HitComponent :type Primitive%20Component%20Object%20Reference) (OtherActor :type Actor%20Object%20Reference) (OtherComp :type Primitive%20Component%20Object%20Reference) (NormalImpulse :type Vector :default "0, 0, 0") (Hit :type Hit%20Result%20Structure%20%28by%20ref%29))
  (bind (_bblockinghit _binitialoverlap _time _distance _location _impactpoint _normal _impactnormal _physmat _hitactor _hitcomponent) (Collision|BreakHitResult Hit))
  (bind (_x _y) (Math|Vector|BreakVector _impactpoint))
  (bind _returnvalue (Math|Vector|MakeVector _x _y 0.0))
  (Class|AProjectile|SpawnImpactFX _impactpoint _impactnormal)
  (Class|AProjectile|SpawnDecalatHitLocation _returnvalue (- (Math|Vector|MakeVector _x _y 1.0) _returnvalue) _hitcomponent)
  (for _array_element (Collision|GetOverlappingActors (Variables|Default|GetSphere) "/Game/BP/Enemy/BP_BaseEnemy.BP_BaseEnemy_C" :!class /Script/Engine.PrimitiveComponent)
    (bind _asbp_base_enemy (Utilities|Casting|CastToBP_BaseEnemy _array_element))
    (Class|BaseEnemy|ApplyDamage _asbp_base_enemy (Variables|Default|GetDamage)))
  (Actor|DestroyActor))

(event EventSpawnDecalatHitLocation
  (params (ImpactLocation :type Vector :default "0, 0, 0") (ImpactNormal :type Vector :default "0, 0, 0") (AttachComponent :type Primitive%20Component%20Object%20Reference))
  (bind _returnvalue (Math|Rotator|MakeRotfromY ImpactNormal))
  (bind (_roll _pitch _yaw) (Math|Rotator|BreakRotator _returnvalue))
  (Class|GameplayStatics|SpawnDecalAttached (Variables|Default|GetDynamicPaintMaterial) (Variables|Default|GetDecalSize) AttachComponent "None" ImpactLocation (Math|Rotator|MakeRotator _roll (- _pitch 9e+01) _yaw) "KeepRelativeOffset" 0.0))

(event EventSpawnImpactFX
  (params (ImpactLocation :type Vector :default "0, 0, 0") (ImpactNormal :type Vector :default "0, 0, 0"))
  (Niagara|SpawnSystematLocation "/Game/Assets/VFX/Explosion/E_Explosion_System.E_Explosion_System" ImpactLocation (Math|Rotator|MakeRotator 0.0 0.0 0.0)))

(fn ConstructionScript)