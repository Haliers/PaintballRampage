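; Shotgun weapon Blueprint that fires spread pellets, leaving paint decals and colored impact effects without applying damage itself.
; Fire takes the character's aim hit point, then runs one Visibility line trace per pellet from the BulletSpawn socket with randomized pitch and yaw spread.
; Each hit spawns a decal and Niagara impact.
; Firing also decreases ammo, spawns a pellet-count-driven muzzle flash, and emits a "Gunshot" noise for AI hearing.
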(event EventBeginPlay)

(event Collision|EventActorBeginOverlap
  (params (OtherActor :type Actor%20Object%20Reference)))

(event EventTick
  (params (DeltaSeconds :type Float%20%28single-precision%29)))

(event EventSpawnMuzzleFlash
  (bind _muzzlescenecomponent (Variables|Default|GetMuzzleSceneComponent))
  (bind _returnvalue (Niagara|SpawnSystematLocation "/Game/Assets/VFX/Shotgun/N_ShotgunEmitter_System.N_ShotgunEmitter_System" (Transformation|GetWorldLocation _muzzlescenecomponent) (Transformation|GetWorldRotation _muzzlescenecomponent)))
  (Effects|Components|ParticleSystem|SetIntParameter _returnvalue "Pellets" (Variables|Default|GetPellets))
  (Effects|Components|ParticleSystem|SetColorParameter _returnvalue "Color" (Variables|Default|GetLinearColor)))

(event EventFire
  (bind _returnvalue (Game|GetPlayerCharacter 0))
  (bind _returnvalue_2 (Class|Weapon|GetHitResultfromCharacter))
  (CallFunction|SpawnPellets (.Location (Collision|BreakHitResult _returnvalue_2)))
  (Class|Weapon|DecreaseAmmo)
  (CallFunction|SpawnMuzzleFlash)
  (Class|Actor|MakeNoise 1.0 _returnvalue (Transformation|GetActorLocation _returnvalue) 0.0 "Gunshot"))

(event EventSpawnImpactFX
  (params (ImpactLocation :type Vector :default "0, 0, 0") (ImpactNormal :type Vector :default "0, 0, 0"))
  (bind _returnvalue (Niagara|SpawnSystematLocation "/Game/Assets/VFX/Impact/N_Impact_System1.N_Impact_System1" ImpactLocation (Math|Conversions|RotationFromXVector ImpactNormal)))
  (Effects|Components|ParticleSystem|SetColorParameter _returnvalue "Color" (Variables|Default|GetLinearColor))
  (Effects|Components|ParticleSystem|SetFloatParameter _returnvalue "Power" 1e+02)
  (Effects|Components|ParticleSystem|SetIntParameter _returnvalue "ParticleNumber" 5))

(fn ConstructionScript)

(fn SpawnPellets
  (params (Target :type Vector))
  (bind _skeletalmeshcomponent (Variables|Default|GetSkeletalMeshComponent))
  (bind _spreadangle (Variables|Default|GetSpreadAngle))
  (bind _returnvalue (Transformation|GetSocketLocation _skeletalmeshcomponent "BulletSpawn"))
  (bind _returnvalue_2 (* _spreadangle -1.0))
  (bind _returnvalue_3 (Class|Shotgun|GetPellets))
  (for _index (range 1 _returnvalue_3)
    (bind (_outhit _returnvalue_4) (Collision|LineTraceByChannel _returnvalue (+ (Math|Vector|RotateVector (- Target _returnvalue) (Math|Rotator|MakeRotator 0.0 (Math|Random|RandomFloatinRange _returnvalue_2 _spreadangle) (Math|Random|RandomFloatinRange _returnvalue_2 _spreadangle))) _returnvalue) "TraceTypeQuery1" false 0 "None" true "(R=1.000000,G=0.000000,B=0.000000,A=1.000000)" "(R=0.000000,G=1.000000,B=0.000000,A=1.000000)" 1.5))
    (if _returnvalue_4
      (Utilities|FlowControl|Sequence
        (:then_0
          (CallFunction|SpawnDecal (.ImpactPoint (Collision|BreakHitResult _outhit)) (.ImpactNormal (Collision|BreakHitResult _outhit))))
        (:then_1
          (Class|Weapon|SpawnImpactFX (.Location (Collision|BreakHitResult _outhit)) (.ImpactNormal (Collision|BreakHitResult _outhit))))))))

(fn SpawnDecal
  (params (Location :type Vector%20%28by%20ref%29) (Normal :type Vector))
  (bind _returnvalue (Math|Rotator|MakeRotfromY Normal))
  (bind (_roll _pitch _yaw) (Math|Rotator|BreakRotator _returnvalue))
  (Class|GameplayStatics|SpawnDecalAttached (Variables|Default|GetDynamicPaintMaterial) (Variables|Default|GetDecalSize) 0 "None" Location (Math|Rotator|MakeRotator _roll (- _pitch 9e+01) _yaw) "KeepRelativeOffset" 0.0))